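; Endless-runner track tile that populates three lanes at random and extends the track as the player advances.
; On BeginPlay, Obstaclespawn rolls chained float ranges per lane to add child actors at the lane transforms, with some outcomes skipping the remaining lanes.
; When the character overlaps the Box, the game mode spawns another tile.
; After a short delay, the tile adds multiplied points, raises walk speed within a clamp, and destroys itself.
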(event OnComponentBeginOverlap(Box)
  (params (OverlappedComponent :type Primitive%20Component%20Object%20Reference) (OtherActor :type Actor%20Object%20Reference) (OtherComp :type Primitive%20Component%20Object%20Reference) (OtherBodyIndex :type Integer) (bFromSweep :type Boolean) (SweepResult :type Hit%20Result%20Structure%20%28by%20ref%29))
  (Utilities|Casting|CastToThirdPersonCharacter OtherActor)
  (bind _asthird_person_game_mode (Utilities|Casting|CastToThirdPersonGameMode (Game|GetGameMode)))
  (Default|Spawntile _asthird_person_game_mode)
  (Utilities|FlowControl|Delay 0.5)
  (bind _asthird_person_game_mode_2 (Utilities|Casting|CastToThirdPersonGameMode (Game|GetGameMode)))
  (Variables|/Game/ThirdPersonBP/Blueprints/ThirdPersonGameMode.ThirdPersonGameMode_C|SetCurentpoints _asthird_person_game_mode_2 (+ (Variables|/Game/ThirdPersonBP/Blueprints/ThirdPersonGameMode.ThirdPersonGameMode_C|GetCurentpoints _asthird_person_game_mode_2) (* (Variables|/Game/ThirdPersonBP/Blueprints/ThirdPersonGameMode.ThirdPersonGameMode_C|Getpointsmultiplier _asthird_person_game_mode_2) 1)))
  (bind _asthird_person_character (Utilities|Casting|CastToThirdPersonCharacter (Game|GetPlayerCharacter 0)))
  (Variables|/Script/Engine.CharacterMovementComponent|SetMaxWalkSpeed (Variables|/Script/Engine.Character|GetCharacterMovement _asthird_person_character) (Math|Float|Clamp(Float) (* (Class|MovementComponent|GetMaxSpeed (Variables|/Script/Engine.Character|GetCharacterMovement _asthird_person_character)) 1.01) 6e+02 1.2e+03))
  (Actor|DestroyActor))

(event EventBeginPlay
  (CallFunction|Obstaclespawn))

(event Collision|EventActorBeginOverlap
  (params (OtherActor :type Actor%20Object%20Reference)))

(event EventTick
  (params (DeltaSeconds :type Float%20%28single-precision%29)))

(fn ConstructionScript)

(fn Obstaclespawn
  (bind _returnvalue (Math|Random|RandomFloatinRange 0.0 1.0))
  (bind _returnvalue_2 (Math|Random|RandomFloatinRange 0.0 1.0))
  (bind _lane0 (Variables|Default|GetLane0))
  (bind _lane1 (Variables|Default|GetLane1))
  (bind _lane2 (Variables|Default|GetLane2))
  (bind _returnvalue_3 (Transformation|GetRelativeTransform _lane1))
  (bind _returnvalue_4 (Transformation|GetRelativeTransform _lane2))
  (bind _returnvalue_5 (Transformation|GetRelativeTransform _lane0))
  ;[1 1 1] Lane 0
  (bind _output_get (Variables|Default|Setrandom1 (Math|Random|RandomFloatinRange 0.0 1.0)))
  (if (Math|Float|InRange(Float) _output_get 0.1 0.4)
    (AddComponent|AddChildActorComponent false _returnvalue_5)
    ;[1 1 1] Lane 1
    (bind _output_get_2 (Variables|Default|Setrandom2 _returnvalue_2 :!label _label))
    (if (Math|Float|InRange(Float) _output_get_2 0.1 0.4)
      (AddComponent|AddChildActorComponent false _returnvalue_3)
      ;[1 1 1] Lane 2
      (bind _output_get_3 (Variables|Default|Setrandom3 _returnvalue :!label _label_2))
      (if (Math|Float|InRange(Float) _output_get_3 0.1 0.4)
        (AddComponent|AddChildActorComponent false _returnvalue_4)
        (elif (Math|Float|InRange(Float) _output_get_3 0.4 0.5)
          (AddComponent|AddChildActorComponent false _returnvalue_4)
          (elif (Math|Float|InRange(Float) _output_get_3 0.5 0.9)
            (AddComponent|AddChildActorComponent false _returnvalue_4)
            (elif (Math|Float|InRange(Float) _output_get_3 0.9 1.0)
              (AddComponent|AddChildActorComponent false _returnvalue_4)
              (elif (Math|Float|InRange(Float) _returnvalue 0.95 1.0)
                (AddComponent|AddChildActorComponent false _returnvalue_4))))))
      (elif (Math|Float|InRange(Float) _output_get_2 0.4 0.5)
        (AddComponent|AddChildActorComponent false _returnvalue_3)
        (goto _label_2)
        (elif (Math|Float|InRange(Float) _output_get_2 0.5 0.9)
          (AddComponent|AddChildActorComponent false _returnvalue_3)
          (goto _label_2)
          (elif (Math|Float|InRange(Float) _output_get_2 0.9 1.0)
            (AddComponent|AddChildActorComponent false _returnvalue_3)
            (goto _label_2)
            (elif (Math|Float|InRange(Float) _returnvalue_2 0.95 1.0)
              (AddComponent|AddChildActorComponent false _returnvalue_3)
              (else
                (goto _label_2)))))))
    (elif (Math|Float|InRange(Float) _output_get 0.4 0.5)
      (AddComponent|AddChildActorComponent false _returnvalue_5)
      (goto _label)
      (elif (Math|Float|InRange(Float) _output_get 0.5 0.9)
        (AddComponent|AddChildActorComponent false _returnvalue_5)
        (goto _label)
        (elif (Math|Float|InRange(Float) _output_get 0.9 0.95)
          (AddComponent|AddChildActorComponent false _returnvalue_5)
          (goto _label)
          (elif (Math|Float|InRange(Float) _output_get 0.95 1.0)
            (AddComponent|AddChildActorComponent false _returnvalue_5)
            (else
              (goto _label))))))))